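; Waypoint manager that guides BP_CanoeAI actors around a looping course of collision components.
; BeginPlay sends every canoe to the first waypoint, and Tick binds the overlap event on the current waypoint's component each frame, without unbinding.
; A canoe overlap advances one CurrentWaypoint index, shared by all canoes, and sets only that canoe's Destination to the next component, wrapping after the last.
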(event `self.ReceiveBeginPlay`
  (bind _outactors (`GameplayStatics.GetAllActorsOfClass` "/Game/Blueprints/BP_CanoeAI.BP_CanoeAI_C"))
  (for _array_element _outactors
    (set `/Game/Blueprints/BP_CanoeAI.Destination` (`self.CollisionComp1`) _array_element)))

(event `self.ReceiveActorBeginOverlap`
  (params (OtherActor :type "Actor Object Reference")))

(event `self.ReceiveTick`
  (params (DeltaSeconds :type "Float (single-precision)"))
  (add `PrimitiveComponent.OnComponentBeginOverlap` (`KismetArrayLibrary.Array_Get` (`|MakeArray` (`self.CollisionComp1`) (`self.CollisionComp2`) (`self.CollisionComp3`) (`self.CollisionComp4`) (`self.CollisionComp5`) (`self.CollisionComp6`) (`self.CollisionComp7`) (`self.CollisionComp8`) (`self.CollisionComp9`) (`self.CollisionComp10`) (`self.CollisionComp11`) (`self.CollisionComp12`) (`self.CollisionComp13`) (`self.CollisionComp14`) (`self.CollisionComp15`) (`self.CollisionComp16`) (`self.CollisionComp17`) (`self.CollisionComp19`) (`self.CollisionComp20`) (`self.CollisionComp21`) (`self.CollisionComp22`) (`self.CollisionComp23`) (`self.CollisionComp24`) (`self.CollisionComp25`) (`self.CollisionComp26`) (`self.CollisionComp27`) (`self.CollisionComp28`) (`self.CollisionComp29`) (`self.CollisionComp30`) (`self.CollisionComp31`) (`self.CollisionComp`)) (`self.currentWaypoint`)) (delegate `OverlapCurrentWP3`)))

(event `OverlapCurrentWP3`
  (params (OtherActor :type "Actor Object Reference") (OtherComp :type "PrimitiveComponent Object Reference") (OtherBodyIndex :type Integer) (bFromSweep :type Boolean) (SweepResult :type "EngineTypes.HitResult Structure (by ref)"))
  (bind _asbp_canoe_ai (cast `/Game/Blueprints/BP_CanoeAI` OtherActor))
  (if (< (`self.currentWaypoint`) 30)
    (set `self.currentWaypoint` (+ (`self.currentWaypoint`) 1))
    (set `/Game/Blueprints/BP_CanoeAI.Destination` (`KismetArrayLibrary.Array_Get` (`|MakeArray` (`self.CollisionComp1`) (`self.CollisionComp2`) (`self.CollisionComp3`) (`self.CollisionComp4`) (`self.CollisionComp5`) (`self.CollisionComp6`) (`self.CollisionComp7`) (`self.CollisionComp8`) (`self.CollisionComp9`) (`self.CollisionComp10`) (`self.CollisionComp11`) (`self.CollisionComp12`) (`self.CollisionComp13`) (`self.CollisionComp14`) (`self.CollisionComp15`) (`self.CollisionComp16`) (`self.CollisionComp17`) (`self.CollisionComp19`) (`self.CollisionComp20`) (`self.CollisionComp21`) (`self.CollisionComp22`) (`self.CollisionComp23`) (`self.CollisionComp24`) (`self.CollisionComp25`) (`self.CollisionComp26`) (`self.CollisionComp27`) (`self.CollisionComp28`) (`self.CollisionComp29`) (`self.CollisionComp30`) (`self.CollisionComp31`) (`self.CollisionComp`)) (`self.currentWaypoint`)) _asbp_canoe_ai)
    (else
      (set `self.currentWaypoint` 0)
      (set `/Game/Blueprints/BP_CanoeAI.Destination` (`self.CollisionComp1`) _asbp_canoe_ai))))

(fn `UserConstructionScript`)