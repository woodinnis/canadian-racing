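; Per-racer lap and checkpoint tracker for a canoe race, bound to one owner vehicle.
; When the owner leaves its single trigger box, the box jumps along 14 checkpoints with a one-second re-trigger lockout.
; The last checkpoint increments the lap, then either resets the box or prints a win message.
; Tick computes distance to the next checkpoint and pushes race progress to the owning BP_Canoe or BP_CanoeAI.
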(event `self.ReceiveActorBeginOverlap`
  (params (OtherActor :type "Actor Object Reference")))

(event `self.ReceiveTick`
  (params (DeltaSeconds :type "Float (single-precision)"))
  ;[1 1 1] Initial Setup
  (`self.Cast To Player` (`self.LAP`) (`self.MAXLAPS`))
  (set `self.distanceToNextCheckpoint` (`KismetMathLibrary.VSize` (- (`SceneComponent.K2_GetComponentLocation` (`self.pOwner`)) (`SceneComponent.K2_GetComponentLocation` (`KismetArrayLibrary.Array_Get` (`|MakeArray` (`self.CP_1`) (`self.CP_2`) (`self.CP_3`) (`self.CP_4`) (`self.CP_5`) (`self.CP_6`) (`self.CP_7`) (`self.CP_8`) (`self.CP_9`) (`self.CP_10`) (`self.CP_11`) (`self.CP_12`) (`self.CP_13`) (`self.CP_14`)) (`self.CP_Count`))))))
  (`KismetSystemLibrary.PrintText` "Hello"))

(event `self.ReceiveBeginPlay`
  ;[1 1 1] Initial Setup
)

(event `self.CP_TriggerBox.OnComponentEndOverlap`
  (params (OtherActor :type "Actor Object Reference") (OtherComp :type "PrimitiveComponent Object Reference") (OtherBodyIndex :type Integer))
  (bind _maxlaps (`self.MAXLAPS`))
  (bind _aswheeled_vehicle (cast `WheeledVehicle` OtherActor))
  (if (== _aswheeled_vehicle (`self.pOwner`))
    (if (== (`self.CP_Count`) 14)
      (`KismetSystemLibrary.Delay` 0.2)
      (set `self.CP_Count` 1)
      (bind _output_get (set `self.LAP` (+ (`self.LAP`) 1)))
      (`self.Cast To Player` _output_get _maxlaps)
      (if (<= (`self.LAP`) _maxlaps)
        (`KismetSystemLibrary.PrintText` "MOVING CP TO FIRST")
        ;[1 1 1] Move Triggerbox to Starting Checkpoint
        (`SceneComponent.K2_SetWorldLocation` (`self.CP_TriggerBox`) (`SceneComponent.K2_GetComponentLocation` (`self.CP_1`)) false)
        (else
          (`KismetSystemLibrary.PrintText` "YOU ARE WINNDER!")))
      (else
        (`/Engine/EditorBlueprintResources/StandardMacros.DoOnce` false :!label _label
          (:`Completed`
            (`SceneComponent.K2_SetWorldLocation` (`self.CP_TriggerBox`) (`SceneComponent.K2_GetComponentLocation` (`KismetArrayLibrary.Array_Get` (`|MakeArray` (`self.CP_1`) (`self.CP_2`) (`self.CP_3`) (`self.CP_4`) (`self.CP_5`) (`self.CP_6`) (`self.CP_7`) (`self.CP_8`) (`self.CP_9`) (`self.CP_10`) (`self.CP_11`) (`self.CP_12`) (`self.CP_13`) (`self.CP_14`)) (`self.CP_Count`))) false)
            (set `self.CP_Count` (+ (`self.CP_Count`) 1))
            (`KismetSystemLibrary.Delay` 1.0)
            (goto _label :!via `Reset`)))))))

(fn `Cast To Player`
  (params (`Current Lap` :type Integer :default 0) (`Total Laps` :type Integer :default 0))
  (bind _cp_count (`self.CP_Count`))
  (bind _totalcheckpoints (`self.totalCheckpoints`))
  (bind _powner (`self.pOwner`))
  (bind _distancetonextcheckpoint (`self.distanceToNextCheckpoint`))
  (bind _asbp_canoe (cast `/Game/Vehicles/CanoeKart/BP_Canoe` _powner)
    (:`then`
      (set `/Game/Vehicles/CanoeKart/BP_Canoe.CurrentLap` `Current Lap` _asbp_canoe)
      (set `/Game/Vehicles/CanoeKart/BP_Canoe.TotalLaps` `Total Laps` _asbp_canoe)
      (set `/Game/Vehicles/CanoeKart/BP_Canoe.currentCheckpoint` _cp_count _asbp_canoe)
      (set `/Game/Vehicles/CanoeKart/BP_Canoe.totalCheckpoints` _totalcheckpoints _asbp_canoe)
      (set `/Game/Vehicles/CanoeKart/BP_Canoe.distanceToNextCheckpoint` _distancetonextcheckpoint _asbp_canoe))
    (:`CastFailed`
      (bind _asbp_canoe_ai (cast `/Game/Blueprints/BP_CanoeAI` _powner))
      (set `/Game/Blueprints/BP_CanoeAI.CurrentLap` `Current Lap` _asbp_canoe_ai)
      (set `/Game/Blueprints/BP_CanoeAI.TotalLaps` `Total Laps` _asbp_canoe_ai)
      (set `/Game/Blueprints/BP_CanoeAI.currentCheckpoint` _cp_count _asbp_canoe_ai)
      (set `/Game/Blueprints/BP_CanoeAI.totalCheckpoints` _totalcheckpoints _asbp_canoe_ai)
      (set `/Game/Blueprints/BP_CanoeAI.distanceToNextCheckpoint` _distancetonextcheckpoint _asbp_canoe_ai))))

(fn `UserConstructionScript`)