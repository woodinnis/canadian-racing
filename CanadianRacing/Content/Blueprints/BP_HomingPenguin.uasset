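; BP_HomingPenguin is an exploding projectile actor that can home in on a target component.
; The Homing event takes a target and, if it is valid, turns on ProjectileMovement homing with a high fixed acceleration.
; A sphere hit or any actor overlap feeds a shared DoOnce that fires the ExplosionForce impulse, spawns the explosion particle effect there and destroys the actor.
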(event `self.ReceiveBeginPlay`)

(event `self.SphereCollision.OnComponentHit`
  (params (OtherActor :type "Actor Object Reference") (OtherComp :type "PrimitiveComponent Object Reference") (NormalImpulse :type "Object.Vector Structure") (Hit :type "EngineTypes.HitResult Structure (by ref)"))
  (bind _explosionforce (`self.ExplosionForce`))
  ;[1 1 1] Explode on Contact
  (`/Engine/EditorBlueprintResources/StandardMacros.DoOnce` false :!label _label
    (:`Completed`
      (`RadialForceComponent.FireImpulse` _explosionforce)
      (`GameplayStatics.SpawnEmitterAtLocation` "/Game/Emitters/Particles/P_Explosion.P_Explosion" (`SceneComponent.K2_GetComponentLocation` _explosionforce))
      (`self.K2_DestroyActor`))))

(event `self.ReceiveActorBeginOverlap`
  (params (OtherActor :type "Actor Object Reference"))
  (goto _label))

(event `self.ReceiveTick`
  (params (DeltaSeconds :type "Float (single-precision)")))

(event `Homing`
  (params (TargetToHit :type "SkeletalMeshComponent Object Reference"))
  (bind _projectilemovement (`self.ProjectileMovement`))
  ;[1 1 1] Set Homing Component
  (if (`KismetSystemLibrary.IsValid` TargetToHit)
    (set `ProjectileMovementComponent.HomingTargetComponent` TargetToHit _projectilemovement)
    (set `ProjectileMovementComponent.bIsHomingProjectile` true _projectilemovement)
    (set `ProjectileMovementComponent.HomingAccelerationMagnitude` 25000.0 _projectilemovement)))

(fn `UserConstructionScript`)