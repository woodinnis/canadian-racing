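; Test AI canoe that drives at constant full throttle and tracks where the player pawn sits relative to it.
; BeginPlay caches itself as BP_Canoe without calling the parent BeginPlay.
; Each Tick, dot products against the mesh's forward and right vectors set Ahead and OnLeft for the player's position, with debug text.
; Neither flag drives steering; the SetSteeringInput node is unconnected.
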(event `self.ReceiveBeginPlay`
  (bind _asbp_canoe (cast `/Game/Vehicles/CanoeKart/BP_Canoe` self)))

(event `self.ReceiveActorBeginOverlap`
  (params (OtherActor :type "Actor Object Reference")))

(event `self.ReceiveTick`
  (params (DeltaSeconds :type "Float (single-precision)"))
  (bind _mesh (`self.Mesh`))
  (bind _mesh_2 (`self.Mesh`))
  (`parent.ReceiveTick` 0.0)
  (`|ExecutionSequence`
    (:`then_0`
      (`WheeledVehicleMovementComponent.SetThrottleInput` (stale `self.ReceiveBeginPlay` _asbp_canoe) 1.0))
    (:`then_1`
      (if (<= (`KismetMathLibrary.Dot_VectorVector` (`KismetMathLibrary.Normal` (`SceneComponent.GetForwardVector` _mesh)) (`KismetMathLibrary.Normal` (- (`SceneComponent.K2_GetComponentLocation` _mesh) (`self.K2_GetActorLocation` (`GameplayStatics.GetPlayerPawn` 0))))) 0.0)
        (`KismetSystemLibrary.PrintText` "DEBUG: AHEAD")
        (set `self.ahead` true)
        (else
          (`KismetSystemLibrary.PrintText` "DEBUG: BEHIND")
          (set `self.ahead` false))))
    (:`then_2`
      (if (<= (`KismetMathLibrary.Dot_VectorVector` (`KismetMathLibrary.Normal` (`SceneComponent.GetRightVector` _mesh_2)) (`KismetMathLibrary.Normal` (- (`SceneComponent.K2_GetComponentLocation` _mesh_2) (`self.K2_GetActorLocation` (`GameplayStatics.GetPlayerPawn` 0))))) 0.0)
        (`KismetSystemLibrary.PrintText` "DEBUG: RIGHT")
        (set `self.onLeft` false)
        (else
          (`KismetSystemLibrary.PrintText` "DEBUG: LEFT")
          (set `self.onLeft` true))))))

(fn `UserConstructionScript`
  (`parent.UserConstructionScript`))