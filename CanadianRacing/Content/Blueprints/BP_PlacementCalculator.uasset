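; Race placement manager that ranks player and AI canoes every tick.
; On BeginPlay it gathers all WheeledVehicle actors, then scores each from lap, checkpoint and distance to the next checkpoint.
; An insertion-sort style pass orders the array by descending score, reading the neighbor's score only once before shifting.
; Each canoe's PLACE is then set from its array index, with casts handling BP_Canoe and BP_CanoeAI separately.
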(event `self.ReceiveBeginPlay`
  (bind _outactors (`GameplayStatics.GetAllActorsOfClass` "/Script/Engine.WheeledVehicle"))
  (set `self.All Vehicles` _outactors))

(event `self.ReceiveActorBeginOverlap`
  (params (OtherActor :type "Actor Object Reference")))

(event `self.ReceiveTick`
  (params (DeltaSeconds :type "Float (single-precision)"))
  (bind _all_vehicles (`self.All Vehicles`))
  (`|ExecutionSequence`
    (:`then_0`
      (for _array_element _all_vehicles
        (`self.Calculate Placement` _array_element)))
    (:`then_1`
      (`self.Sort Vehicles into Place`)
      (for (_array_element_2 _array_index) _all_vehicles
        (bind _asbp_canoe (cast `/Game/Vehicles/CanoeKart/BP_Canoe` _array_element_2)
          (:`then`
            (bind _returnvalue (+ _array_index 1))
            (set `/Game/Vehicles/CanoeKart/BP_Canoe.PLACE` _returnvalue _asbp_canoe))
          (:`CastFailed`
            (bind _asbp_canoe_ai (cast `/Game/Blueprints/BP_CanoeAI` _array_element_2))
            (set `/Game/Blueprints/BP_CanoeAI.PLACE` _returnvalue _asbp_canoe_ai)))))))

(fn `Calculate Placement`
  (params (Vehicle :type "WheeledVehicle Object Reference"))
  (bind _asbp_canoe (cast `/Game/Vehicles/CanoeKart/BP_Canoe` Vehicle)
    (:`then`
      (set `/Game/Vehicles/CanoeKart/BP_Canoe.placementScore` (- (* (+ (`/Game/Vehicles/CanoeKart/BP_Canoe.currentCheckpoint` _asbp_canoe) (* (`/Game/Vehicles/CanoeKart/BP_Canoe.totalCheckpoints` _asbp_canoe) (- (`/Game/Vehicles/CanoeKart/BP_Canoe.CurrentLap` _asbp_canoe) 1))) 10) (`KismetMathLibrary.FFloor` (* (`/Game/Vehicles/CanoeKart/BP_Canoe.distanceToNextCheckpoint` _asbp_canoe) 0.001))) _asbp_canoe))
    (:`CastFailed`
      (bind _asbp_canoe_ai (cast `/Game/Blueprints/BP_CanoeAI` Vehicle))
      (set `/Game/Blueprints/BP_CanoeAI.placementScore` (- (* (+ (`/Game/Blueprints/BP_CanoeAI.currentCheckpoint` _asbp_canoe_ai) (* (`/Game/Blueprints/BP_CanoeAI.totalCheckpoints` _asbp_canoe_ai) (- (`/Game/Blueprints/BP_CanoeAI.CurrentLap` _asbp_canoe_ai) 1))) 10) (`KismetMathLibrary.FFloor` (* (`/Game/Blueprints/BP_CanoeAI.distanceToNextCheckpoint` _asbp_canoe_ai) 0.001))) _asbp_canoe_ai))))

(fn `Sort Vehicles into Place`
  (bind _target_index_stepper (`self.Target Index Stepper`))
  (bind _item (`KismetArrayLibrary.Array_Get` (`self.All Vehicles`) (- _target_index_stepper 1)))
  (for (_array_element _array_index) (`self.All Vehicles`)
    (bind _output_get (set `self.Target Current Element` _array_element))
    (bind _asbp_canoe (cast `/Game/Vehicles/CanoeKart/BP_Canoe` _output_get)
      (:`then`
        (set `self.Target Placement Score` (`/Game/Vehicles/CanoeKart/BP_Canoe.placementScore` _asbp_canoe)))
      (:`CastFailed`
        (bind _asbp_canoe_ai (cast `/Game/Blueprints/BP_CanoeAI` _array_element))
        (set `self.Target Placement Score` (`/Game/Blueprints/BP_CanoeAI.placementScore` _asbp_canoe_ai))))
    (set `self.Target Index Stepper` _array_index)
    (bind _asbp_canoe_ai_2 (cast `/Game/Blueprints/BP_CanoeAI` _item)
      (:`then`
        (set `self.Second Target Placement Score` (`/Game/Blueprints/BP_CanoeAI.placementScore` _asbp_canoe_ai_2)))
      (:`CastFailed`
        (bind _asbp_canoe_2 (cast `/Game/Vehicles/CanoeKart/BP_Canoe` _item))
        (set `self.Second Target Placement Score` (`/Game/Vehicles/CanoeKart/BP_Canoe.placementScore` _asbp_canoe_2))))
    (while (and (> (`self.Target Placement Score`) (`self.Second Target Placement Score`)) (> _target_index_stepper 0))
      (`KismetArrayLibrary.Array_Set` (`self.All Vehicles`) (`self.Target Index Stepper`) (`KismetArrayLibrary.Array_Get` (`self.All Vehicles`) (- (`self.Target Index Stepper`) 1)))
      (set `self.Target Index Stepper` (- (`self.Target Index Stepper`) 1)))
    (`KismetArrayLibrary.Array_Set` (`self.All Vehicles`) (`self.Target Index Stepper`) (`self.Target Current Element`))))

(fn `UserConstructionScript`)