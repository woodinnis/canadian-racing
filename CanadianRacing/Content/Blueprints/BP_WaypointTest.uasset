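; BP_WaypointTest is a looping waypoint course that steers BP_CanoeAI actors through nine collision components.
; On BeginPlay it sets every canoe's Destination to the first component.
; Tick binds the current component's overlap event without unbinding earlier ones; a canoe overlap advances the index, wrapping after the last, and retargets that canoe.
; One index is shared by all canoes, and non-canoe overlaps print a debug message.
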(event `self.ReceiveBeginPlay`
  (bind _outactors (`GameplayStatics.GetAllActorsOfClass` "/Game/Blueprints/BP_CanoeAI.BP_CanoeAI_C"))
  (for _array_element _outactors
    (set `/Game/Blueprints/BP_CanoeAI.Destination` (`self.CollisionComp`) _array_element)))

(event `self.ReceiveActorBeginOverlap`
  (params (OtherActor :type "Actor Object Reference")))

(event `self.ReceiveTick`
  (params (DeltaSeconds :type "Float (single-precision)"))
  (add `PrimitiveComponent.OnComponentBeginOverlap` (`KismetArrayLibrary.Array_Get` (`|MakeArray` (`self.CollisionComp`) (`self.CollisionComp1`) (`self.CollisionComp2`) (`self.CollisionComp3`) (`self.CollisionComp4`) (`self.CollisionComp5`) (`self.CollisionComp6`) (`self.CollisionComp7`) (`self.CollisionComp8`)) (`self.currentWaypoint`)) (delegate `Overlap Current Waypoint`)))

(event `Overlap Current Waypoint`
  (params (OtherActor :type "Actor Object Reference") (OtherComp :type "PrimitiveComponent Object Reference") (OtherBodyIndex :type Integer) (bFromSweep :type Boolean) (SweepResult :type "EngineTypes.HitResult Structure (by ref)"))
  (bind _asbp_canoe_ai (cast `/Game/Blueprints/BP_CanoeAI` OtherActor)
    (:`then`
      (if (< (`self.currentWaypoint`) 8)
        (set `self.currentWaypoint` (+ (`self.currentWaypoint`) 1))
        (set `/Game/Blueprints/BP_CanoeAI.Destination` (`KismetArrayLibrary.Array_Get` (`|MakeArray` (`self.CollisionComp`) (`self.CollisionComp1`) (`self.CollisionComp2`) (`self.CollisionComp3`) (`self.CollisionComp4`) (`self.CollisionComp5`) (`self.CollisionComp6`) (`self.CollisionComp7`) (`self.CollisionComp8`)) (`self.currentWaypoint`)) _asbp_canoe_ai)
        (else
          (set `self.currentWaypoint` 0)
          (set `/Game/Blueprints/BP_CanoeAI.Destination` (`self.CollisionComp`) _asbp_canoe_ai))))
    (:`CastFailed`
      (`KismetSystemLibrary.PrintText` "Hello"))))

(fn `UserConstructionScript`)