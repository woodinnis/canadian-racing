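; Boost pad that gives player and AI canoes a forward shove when they overlap its Trigger component.
; The overlap casts to BP_Canoe, then BP_CanoeAI, and applies a one-shot, mass-dependent impulse along that canoe's forward vector, scaled by ThrustScale.
; AI canoes get a larger hard-coded multiplier than the player canoe.
; Leftover disconnected nodes that boost the player pawn directly never run.
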(event `self.ReceiveBeginPlay`)

(event `self.Trigger.OnComponentBeginOverlap`
  (params (OtherActor :type "Actor Object Reference") (OtherComp :type "PrimitiveComponent Object Reference") (OtherBodyIndex :type Integer) (bFromSweep :type Boolean) (SweepResult :type "EngineTypes.HitResult Structure (by ref)"))
  (bind _asbp_canoe (cast `/Game/Vehicles/CanoeKart/BP_Canoe` OtherActor)
    (:`then`
      (`PrimitiveComponent.AddImpulse` _asbp_canoe (* (`KismetMathLibrary.Normal` (`self.GetActorForwardVector` _asbp_canoe)) (* (`self.Thrust Scale`) 1000000.0)) "None" false))
    (:`CastFailed`
      (bind _asbp_canoe_ai (cast `/Game/Blueprints/BP_CanoeAI` OtherActor))
      (`PrimitiveComponent.AddImpulse` _asbp_canoe_ai (* (`KismetMathLibrary.Normal` (`SceneComponent.GetForwardVector` _asbp_canoe_ai)) (* (`self.Thrust Scale`) 1900000.0)) "None" false))))

(event `self.ReceiveTick`
  (params (DeltaSeconds :type "Float (single-precision)")))

(fn `UserConstructionScript`)