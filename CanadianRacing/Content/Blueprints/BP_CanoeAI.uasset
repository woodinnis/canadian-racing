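; AI-driven racing canoe vehicle that steers toward a Destination at full throttle and rights itself when tipped over.
; Each Tick sets steering from a right-vector dot product, runs a delayed auto-flip, and calls SpawnCheckpoints, which spawns level-specific checkpoints whenever LevelInstantiated is true, with no reset.
; Helper functions, uncalled here, cover start countdown and headstart boost, shunt gauge regen, penguin ammo, nearest-vehicle homing and invulnerability.
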(event `self.ReceiveTick`
  (params (DeltaSeconds :type "Float (single-precision)"))
  (bind _updatedprimitive (`MovementComponent.UpdatedPrimitive` (`self.VehicleMovement`)))
  (bind _returnvalue (`KismetMathLibrary.DegAcos` (`KismetMathLibrary.Dot_VectorVector` (`KismetMathLibrary.Normal` (`SceneComponent.GetUpVector` (`self.Mesh`))) (`KismetMathLibrary.MakeVector` 0.0 0.0 1.0))))
  (bind _returnvalue_2 (>= _returnvalue 90.0))
  (`|ExecutionSequence`
    (:`then_0`
      (`self.Movement`))
    (:`then_1`
      ;[1 1 1] Functions
      ;;[1 1 1] Auto Flip
      (if _returnvalue_2
        (`KismetSystemLibrary.Delay` (`self.Flip Timer`))
        (if _returnvalue_2
          (`|ExecutionSequence`
            (:`then_0`
              (`SceneComponent.K2_AddRelativeLocation` _updatedprimitive (`KismetMathLibrary.MakeVector` 0.0 0.0 200.0) false))
            (:`then_1`
              (`SceneComponent.K2_AddLocalRotation` _updatedprimitive (`KismetMathLibrary.MakeRot` 0.0 0.0 _returnvalue) false))))))
    (:`then_2`
      (`self.SpawnCheckpoints`))))

(event `self.ReceiveBeginPlay`)

(fn `DetermineHomingTarget`
  (for (_array_element _array_index) (`self.VehiclesToTarget`)
    (if (`KismetSystemLibrary.IsValid` _array_element)
      (bind _returnvalue (`KismetMathLibrary.VSize` (- (`SceneComponent.K2_GetComponentLocation` (`self.Mesh`)) (`SceneComponent.K2_GetComponentLocation` _array_element))))
      (if (< _returnvalue (`self.TargetDistance`))
        (set `self.TargetDistance` _returnvalue)
        (set `self.TargetIndex` _array_index))))
  (set `self.Homing Target` (`WheeledVehicle.Mesh` (`KismetArrayLibrary.Array_Get` (`self.VehiclesToTarget`) (`self.TargetIndex`))))
  (set `self.TargetDistance` 100000000.0))

(fn `Gauge Regen`
  (bind _max_gauge (`self.Max Gauge`))
  ;[1 1 1] If maxed, set to max
  (if (>= (`self.Shunt Gauge`) _max_gauge)
    (bind _output_get (set `self.Shunt Gauge` _max_gauge))
    (else
      ;[1 1 1] Regen if not max
      (bind _output_get_2 (set `self.Shunt Gauge` (+ (stale _output_get_2) (`self.Gauge Regen Rate`)))))))

(fn `GetInvulnerable`
  (returns (isInvulnerable :type Boolean))
  (return (`self.isInvulnerable`)))

(fn `IncrementPenguinAmmo`
  (set `self.PenguinAmmo` (+ (`self.PenguinAmmo`) 1)))

(fn `IncrementPenguinCDAmmo`
  (set `self.PenguinShuntCDAmmo` (+ (`self.PenguinShuntCDAmmo`) 1)))

(fn `IncrementSuicidePenguinAmmo`
  (set `self.SuicidePenguinAmmo` (+ (`self.SuicidePenguinAmmo`) 1)))

(fn `Movement`
  (bind _mesh (`self.Mesh`))
  (bind _mesh_2 (`self.Mesh`))
  (`|ExecutionSequence`
    (:`then_0`
      ;[1 1 1] Determine if target is ahead or behind (USE WAYPOINT INSTEAD OF PLAYER ACTOR LOCATION)
      (if (<= (`KismetMathLibrary.Dot_VectorVector` (`KismetMathLibrary.Normal` (`SceneComponent.GetForwardVector` _mesh)) (`KismetMathLibrary.Normal` (- (`SceneComponent.K2_GetComponentLocation` _mesh) (`SceneComponent.K2_GetComponentLocation` (`self.Destination`))))) 0.0)
        (`WheeledVehicleMovementComponent.SetThrottleInput` 1.0)
        (else
          (`WheeledVehicleMovementComponent.SetThrottleInput` 1.0))))
    (:`then_1`
      ;[1 1 1] Determine if target is left or right (USE WAYPOINT INSTEAD OF PLAYER ACTOR LOCATION)
      (`WheeledVehicleMovementComponent.SetSteeringInput` (* (`KismetMathLibrary.Dot_VectorVector` (`KismetMathLibrary.Normal` (`SceneComponent.GetRightVector` _mesh_2)) (`KismetMathLibrary.Normal` (- (`SceneComponent.K2_GetComponentLocation` _mesh_2) (`SceneComponent.K2_GetComponentLocation` (`self.Destination`))))) -1.0)))))

(fn `SetInvulnerable`
  (params (isInvulnerable :type Boolean :default false))
  (set `self.isInvulnerable` isInvulnerable))

(fn `SpawnCheckpoints`
  (bind _asmy_player_controller (cast `/Game/UI/Menus/MenuMP/MyPlayerController` (`GameplayStatics.GetPlayerController` 0))
    (:`then`
      (if (`/Game/UI/Menus/MenuMP/MyPlayerController.Level Instantiated` _asmy_player_controller)
        (switch `string` (`/Game/UI/Menus/MenuMP/MyPlayerController.Current Level` _asmy_player_controller)
          (:`Brett`
            ;[1 1 1] Load Brett Checkpoints
            ;;[1 1 1] Should check which current level
            (bind _returnvalue (`|SpawnActorFromClass` "/Game/Blueprints/BP_BrettCheckpoints.BP_BrettCheckpoints_C" (`KismetMathLibrary.MakeTransform` (2669.0 -2613.0 -618.0))))
            (set `/Game/Blueprints/BP_BrettCheckpoints.pOwner` self _returnvalue))
          (:`Caleb`
            ;[1 1 1] Load 'Caleb' Checkpoints
            (bind _returnvalue_2 (`|SpawnActorFromClass` "/Game/Blueprints/BP_CalebCheckpoints.BP_CalebCheckpoints_C" (`KismetMathLibrary.MakeTransform` (-1770.0 -11990.0 25.0))))
            (set `/Game/Blueprints/BP_CalebCheckpoints.pOwner` self _returnvalue_2)))))
    (:`CastFailed`
      (`KismetSystemLibrary.PrintText` "CAST FAILED"))))

(fn `StartCounter`
  (if (> (`self.StartCount`) 0.0)
    (bind _output_get (set `self.StartCount` (- (stale _output_get) 0.1)))
    (bind _output_get_2 (set `self.RaceTime` (+ (stale _output_get_2) 0.1) :!label _label))
    (else
      (`|ExecutionSequence`
        (:`then_0`
          (goto _label))
        (:`then_1`
          (`/Engine/EditorBlueprintResources/StandardMacros.DoOnce` false
            (:`Completed`
              (set `self.RaceState` 1)
              (set `self.StartCount` 0.0))))))))

(fn `StateCheck`
  (params (Accel :type "Float (double-precision)" :default 0.0))
  (bind _mesh (`self.Mesh`))
  (bind _startcount (`self.StartCount`))
  ;[1 1 1] Checking State
  (switch `int` (`self.RaceState`)
    (:`0`
      ;[1 1 1] Headstart or Slowstart
      (if (and (> Accel 0.0) (`self.CanStartBonus`))
        (if (and (<= _startcount (`self.Max_Boost_Window`)) (>= _startcount (`self.Min_Boost_Window`)))
          (set `self.Headstart` true)
          (else
            (set `self.Headstart` false)))
        (set `self.CanStartBonus` false)))
    (:`1`
      ;[1 1 1] Apply Head/Slowstart effects
      (if (>= (`self.RaceTime`) 7.0)
        (set `self.Headstart` false)
        (elif (`self.Headstart`)
          (`PrimitiveComponent.AddForce` _mesh (* (`SceneComponent.GetForwardVector` _mesh) 1000000.0) "None"))))))

(fn `UserConstructionScript`)